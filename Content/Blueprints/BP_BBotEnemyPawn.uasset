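; Enemy bot pawn that wires its animation, melee ability and overhead widgets together at BeginPlay.
; It caches the BPA_EnemyBot anim instance to forward animation-played events, and passes HitStart to the melee ability for linecasts.
; Health bar, spring arm and ability display use absolute rotation, with the health bar fed by HealthComponent.
; The ability widget runs in non-player mode and receives abilities two frames after each enemy data update.
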(event OnAnimationPlayed(AnimationComponent)
  ;[0.15 0.15 0.15 0.5] Call Anim Play event in Animation Blueprint
  (Default|OnAnimPlay (Variables|Default|GetAnim%20Blueprint)))

(event Custom|OnEnemyData
  (params (enemyData :type Enemy%20Data%20Structure))
  ;[0.15 0.15 0.15 0.5] Ability Equip Widget
  (Utilities|FlowControl|DelayUntilNextFrame)
  (Utilities|FlowControl|DelayUntilNextFrame)
  (Default|SetPlayerAbilities (Variables|Default|GetAs%20WBP%20Ability%20Equip) (Utilities|Struct|BreakEnemyData enemyData)))

(event EventBeginPlay
  ;[0.15 0.15 0.15 0.5] Set Anim Blueprint
  (bind _asbpa_enemy_bot (Utilities|Casting|CastToBPA_EnemyBot (Components|SkeletalMesh|GetAnimInstance (Variables|Default|GetSkeletalMesh))))
  (Variables|Default|SetAnim%20Blueprint _asbpa_enemy_bot)
  ;[0.15 0.15 0.15 0.5] Set HitStart for melee linecast
  (Variables|/Script/BBattle.MeleeAttackAbility|SethitStart (Variables|Default|GetMeleeAttackAbility) (Variables|Default|GethitStart))
  ;[0.15 0.15 0.15 0.5] Health Bar Component
  (Variables|/Script/Engine.SceneComponent|SetbAbsoluteRotation (Variables|Default|GetHealthBar) true)
  (Variables|/Script/Engine.SceneComponent|SetbAbsoluteRotation (Variables|Default|GetSpringArm) true)
  (bind _aswbp_health_bar (Utilities|Casting|CastToWBP_HealthBar (UserInterface|GetWidget (Variables|Default|GetHealthBar))))
  (Default|SetHealthComponent _aswbp_health_bar (Variables|Default|GetHealthComponent))
  ;[0.15 0.15 0.15 0.5] Ability Equip Widget
  (Variables|/Script/Engine.SceneComponent|SetbAbsoluteRotation (Variables|Default|GetAbilityEquip) true)
  (bind _aswbp_ability_equip (Utilities|Casting|CastToWBP_AbilityEquip (UserInterface|GetWidget (Variables|Default|GetAbilityEquip))))
  (Variables|Default|SetAs%20WBP%20Ability%20Equip _aswbp_ability_equip)
  (EventDispatchers|BindEventtoOnEnemyDataUpdated self (delegate Custom|OnEnemyData))
  (Default|StartTickHighlight (Variables|Default|GetAs%20WBP%20Ability%20Equip) (Variables|Default|GetintervalWatch))
  (Variables|/Game/Blueprints/UI/WBP_AbilityEquip.WBP_AbilityEquip_C|SetIsPlayer (Variables|Default|GetAs%20WBP%20Ability%20Equip) false))

(event Collision|EventActorBeginOverlap
  (params (OtherActor :type Actor%20Object%20Reference)))

(event EventTick
  (params (DeltaSeconds :type Float%20%28single-precision%29)))

(fn ConstructionScript)