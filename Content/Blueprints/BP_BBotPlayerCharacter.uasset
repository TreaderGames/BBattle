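; Player character Blueprint for the battle bot, wiring its animation, melee ability and attached health and ability widgets.
; BeginPlay shows the cursor, caches the anim Blueprint, passes HitStart to the melee linecast and gives the spring arm and widgets absolute rotation.
; The health bar binds to HealthComponent, while the ability widget tracks IntervalWatch and refreshes whenever PlayerDataSubSystem reports updated abilities.
; AnimationComponent play events are forwarded to the anim Blueprint.
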(event OnAnimationPlayed(AnimationComponent)
  ;[0.15 0.15 0.15 0.5] Call Anim Play event in Animation Blueprint
  (Default|OnAnimPlay (Variables|Default|GetAnimBlueprint)))

(event Custom|CustomEvent
  ;[0.15 0.15 0.15 0.5] Ability Equip Widget
  (CallFunction|HandleAbilitiesUpdate))

(event EventBeginPlay
  ;[0.15 0.15 0.15 0.5] ShowCursorDefault
  (Variables|/Script/Engine.PlayerController|SetbShowMouseCursor (Game|GetPlayerController 0) true)
  ;[0.15 0.15 0.15 0.5] GetAnimBlueprint
  (bind _asbpa_battle_bot (Utilities|Casting|CastToBPA_BattleBot (Components|SkeletalMesh|GetAnimInstance (Variables|/Script/Engine.Character|GetMesh (Game|GetPlayerCharacter 0)))))
  (Variables|Default|SetAnimBlueprint _asbpa_battle_bot)
  ;[0.15 0.15 0.15 0.5] Set HitStart for melee linecast
  (Variables|/Script/BBattle.MeleeAttackAbility|SethitStart (Variables|Default|GetMeleeAttackAbility) (Variables|Default|GethitStart))
  ;[0.15 0.15 0.15 0.5] Health Bar Widget
  (Variables|/Script/Engine.SceneComponent|SetbAbsoluteRotation (Variables|Default|GetHealthBar) true)
  (Variables|/Script/Engine.SceneComponent|SetbAbsoluteRotation (Variables|Default|GetSpringArm) true)
  (bind _aswbp_health_bar (Utilities|Casting|CastToWBP_HealthBar (UserInterface|GetWidget (Variables|Default|GetHealthBar))))
  (Default|SetHealthComponent _aswbp_health_bar (Variables|Default|GetHealthComponent))
  ;[0.15 0.15 0.15 0.5] Ability Equip Widget
  (Variables|/Script/Engine.SceneComponent|SetbAbsoluteRotation (Variables|Default|GetAbilityEquip) true)
  (bind _aswbp_ability_equip (Utilities|Casting|CastToWBP_AbilityEquip (UserInterface|GetWidget (Variables|Default|GetAbilityEquip))))
  (bind _output_get (Variables|Default|SetAs%20WBP%20Ability%20Equip _aswbp_ability_equip))
  (Variables|/Game/Blueprints/UI/WBP_AbilityEquip.WBP_AbilityEquip_C|SetIsPlayer _output_get true)
  (EventDispatchers|AssignOnAbilitiesUpdated (Subsystems|GetPlayerDataSubSystem) (delegate Custom|CustomEvent))
  (Default|StartTickHighlight (Variables|Default|GetAs%20WBP%20Ability%20Equip) (Variables|Default|GetintervalWatch)))

(fn ConstructionScript)

(fn HandleAbilitiesUpdate
  (bind _returnvalue (Class|PlayerDataSubSystem|GetAbilityArr (Subsystems|GetPlayerDataSubSystem)))
  (Default|SetPlayerAbilities (Variables|Default|GetAs%20WBP%20Ability%20Equip) _returnvalue))